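; BP_Zombie is a melee enemy that chases the player from BeginPlay, speeding up when PawnSensing spots a pawn.
; AI MoveTo, targeting the player controller, retries on failure and starts an attack on success, whose montage notify sphere-overlaps at Arrow1 to damage BP_FirstPersonCharacter.
; Point damage lowers Health and plays a hit reaction, or triggers death, which stops movement, plays a dying montage and disables capsule collision.
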(event `Death`
  ;[0 0 0] Death
  (set `self.IsDeath` true)
  (`NavMovementComponent.StopActiveMovement` (`self.CharacterMovement`))
  (`|PlayMontage` (`self.Mesh`) "/Game/_Main/Zombie/Animations/Montages/ZombieDying_Montage.ZombieDying_Montage"
    (:`then`
      (`PrimitiveComponent.SetCollisionEnabled` (`self.CapsuleComponent`) "NoCollision"))))

(event `self.PawnSensing.OnSeePawn`
  (params (Pawn :type "Pawn Object Reference"))
  ;[0 1 0.9929] Setting Speed
  (set `CharacterMovementComponent.MaxWalkSpeed` 360.0 (`self.CharacterMovement`)))

(event `self.ReceiveBeginPlay`
  ;[0 1 0.0431] Start Run To Player
  (`self.RunToPlayer`))

(event `self.ReceivePointDamage`
  (params (Damage :type "Float (single-precision)") (DamageType :type "DamageType Object Reference") (HitLocation :type "Vector Structure") (HitNormal :type "Vector Structure") (HitComponent :type "PrimitiveComponent Object Reference") (BoneName :type Name) (ShotFromDirection :type "Vector Structure") (InstigatedBy :type "Controller Object Reference") (DamageCauser :type "Actor Object Reference") (HitInfo :type "HitResult Structure (by ref)"))
  ;[1 0 0.8506] Take Dmage
  (if (`self.IsDeath`)
    _
    (elif (<= (`self.Health`) 0.0)
      (`self.Death`)
      (else
        (bind _output_get (set `self.Health` (- (`self.Health`) Damage)))
        (if (<= _output_get 0.0)
          (`self.Death`)
          (else
            (`|PlayMontage` (`self.Mesh`) "/Game/_Main/Zombie/Animations/Montages/ZombieHitMontage.ZombieHitMontage"
              (:`then`
                (`self.RunToPlayer`)))))))))

(event `RunToPlayer`
  ;[1 0 0] Run To Player
  (if (not (`self.IsDeath`))
    (`|AIMoveTo` self (0.0 0.0 0.0) (`GameplayStatics.GetPlayerController` 0) 40.0
      (:`OnSuccess`
        (`self.AttackPlayer`))
      (:`OnFail`
        (`self.RunToPlayer`)))))

(event `AttackPlayer`
  ;[0.1714 0 1] Attack Player
  (`|PlayMontage` (`self.Mesh`) "/Game/_Main/Zombie/Animations/Montages/ZombieAttack_Montage.ZombieAttack_Montage"
    (:`OnCompleted`
      (`self.RunToPlayer`))
    (:`OnNotifyBegin`
      (bind (_outactors _returnvalue) (`KismetSystemLibrary.SphereOverlapActors` (`SceneComponent.K2_GetComponentLocation` (`self.Arrow1`)) 60.0 (`|MakeArray` "ObjectTypeQuery3" :!type "EObjectTypeQuery Enum") "/Game/_Main/Blueprints/BP_FirstPersonCharacter.BP_FirstPersonCharacter_C" (`|MakeArray` self :!type "Actor Object Reference")))
      (if _returnvalue
        (for _array_element _outactors
          (`GameplayStatics.ApplyDamage` _array_element 20.0 (`self.GetController`) self "/Script/Engine.DamageType"))))))

(fn `UserConstructionScript`)